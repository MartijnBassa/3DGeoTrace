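; BP_Wms_Manager manages the opacity of the WMS decals attached to it as components.
; On BeginPlay it creates a dynamic material instance for each DecalComponent, caches them in WmsMaterials and hides them all by setting opacity to zero.
; SetOpacity writes the given value to the Opacity scalar parameter of every cached material, so all decals fade together.
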(event EventBeginPlay
  (for _array_element (Actor|GetComponentsByClass "/Script/Engine.DecalComponent")
    (bind _returnvalue (Rendering|Material|CreateDynamicMaterialInstance _array_element :!class /Script/Engine.DecalComponent))
    (Utilities|Array|Add (Variables|Private|Get_WmsMaterials) _returnvalue))
  (Public|SetOpacity 0.0))

(fn ConstructionScript)

(fn SetOpacity
  (params (Opacity :type Float%20%28double-precision%29))
  (for _array_element (Variables|Private|Get_WmsMaterials)
    (Rendering|Material|SetScalarParameterValue _array_element "Opacity" Opacity :!class /Script/Engine.MaterialInstanceDynamic)))