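; InsightArray is a data-holder Blueprint for a single insight, storing its icon, text, spline point and ID.
; Simple getter and setter functions expose each field, with no other logic in the graphs.
; The ID setter takes no input and assigns a freshly generated GUID, so each call replaces the insight's identity.
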(fn SetInsightIcon
  (params (Icon :type Texture%202D%20Object%20Reference))
  (Variables|Default|SetInsightIcon Icon))

(fn GetInsightIcon
  (return (Variables|Default|GetInsightIcon)))

(fn SetInsightText
  (params (Text :type Text))
  (Variables|Default|SetInsightText Text))

(fn GetInsightText
  (return (Variables|Default|GetInsightText)))

(fn SetSplinePoint
  (params (Point :type Array%20of%20Vectors))
  (Variables|Default|SetInsightPoint Point))

(fn GetSplinePoint
  (return (Variables|Default|GetInsightPoint)))

(fn SetInsightID
  (Variables|Default|SetInsightID (Guid|NewGuid)))

(fn GetInsightID
  (return (Variables|Default|GetInsightID)))