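; Spline-driven Blueprint that lays a chosen static mesh along a spline as deforming spline mesh segments.
; The construction script sets closed-loop from Looping, then adds a segment between consecutive points using world-space locations and tangents.
; The loop stops at the second-last point, so the closing segment gets no mesh even when looping.
; Distance-based start and end helpers are unused and have zeroed spacing and tangent clamps.
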(event EventBeginPlay)

(event Collision|EventActorBeginOverlap
  (params (OtherActor :type Actor%20Object%20Reference)))

(event EventTick
  (params (DeltaSeconds :type Float%20%28single-precision%29)))

(fn ConstructionScript
  (bind _spline (Variables|Default|GetSpline))
  (bind _returnvalue (Spline|GetNumberOfSplinePoints _spline))
  (Spline|SetClosedLoop _spline (Variables|Default|GetLooping) true)
  (for _index (range 0 (- _returnvalue 2))
    (bind _returnvalue_2 (AddComponent|AddSplineMeshComponent false))
    (SplineMesh|SetStartandEnd _returnvalue_2 (.Location (Spline|GetLocationandTangentatSplinePoint _spline _index "World")) (.Tangent (Spline|GetLocationandTangentatSplinePoint _spline _index "World")) (.Location (Spline|GetLocationandTangentatSplinePoint _spline (Math|Integer|%(Integer) (+ _index 1) _returnvalue) "World")) (.Tangent (Spline|GetLocationandTangentatSplinePoint _spline (Math|Integer|%(Integer) (+ _index 1) _returnvalue) "World")) true :!class /Script/Engine.SplineMeshComponent)
    (Components|StaticMesh|SetStaticMesh _returnvalue_2 (Variables|Default|GetStatisMesh))))

(fn GetEndPosTangent
  (params (Index :type Integer))
  (bind _returnvalue (+ Index 1))
  (bind _spline (Variables|Default|GetSpline))
  (bind _returnvalue_2 (* _returnvalue 0.0))
  (return (Spline|GetLocationatDistanceAlongSpline _spline _returnvalue_2 "Local") (Math|Vector|ClampVectorSize (Spline|GetTangentatDistanceAlongSpline _spline _returnvalue_2 "Local") 0.0 0.0)))

(fn GetStartPosTangent
  (params (Index :type Integer))
  (bind _returnvalue (* Index 0.0))
  (bind _spline (Variables|Default|GetSpline))
  (return (Spline|GetLocationatDistanceAlongSpline _spline _returnvalue "Local") (Math|Vector|ClampVectorSize (Spline|GetTangentatDistanceAlongSpline _spline _returnvalue "Local") 0.0 0.0)))