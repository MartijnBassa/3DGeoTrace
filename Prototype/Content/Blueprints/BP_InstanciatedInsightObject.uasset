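; Actor for an insight object in the world, carrying an ID, a point index and a widget that turns to face the player camera.
; On BeginPlay it binds to every top-level UserInterface widget's insight-icon update and relays the insight arrays with its ID through UpdateObjectIcon.
; A looping timer, rather than Tick, re-aims the widget at the camera.
; UpdateInsightIcon is an empty stub.
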(event Custom|Start%20Timer
  (Utilities|Time|SetTimerbyEvent (delegate Custom|Update%20Rotation) 0.1 true))

(event Custom|Update%20Rotation
  (bind _widget (Variables|Default|GetWidget))
  (Transformation|SetWorldRotation _widget (Math|Rotator|FindLookatRotation (Transformation|GetWorldLocation _widget) (Camera|GetCameraLocation (Game|GetPlayerCameraManager 0))) false false))

(event Custom|Update%20Icon
  (params (Insight%20Array :type Array%20of%20BP%20Insight%20Array%20Object%20References) (InsightObjectArray :type Array%20of%20BP%20Instanciated%20Insight%20Object%20Object%20References))
  (Default|CallUpdateObjectIcon Insight%20Array InsightObjectArray (Variables|Default|GetID)))

(event EventBeginPlay
  (Utilities|FlowControl|Sequence
    (:then_0
      (bind _foundwidgets (Widget|GetAllWidgetsOfClass "/Game/UI/UserInterface.UserInterface_C" true))
      (for _array_element _foundwidgets
        (EventDispatchers|BindEventtoUpdateInsightWorldIcon _array_element (delegate Custom|Update%20Icon))))
    (:then_1
      (CallFunction|StartTimer))))

(event Collision|EventActorBeginOverlap
  (params (OtherActor :type Actor%20Object%20Reference)))

(event EventTick
  (params (DeltaSeconds :type Float%20%28single-precision%29)))

(fn ConstructionScript)

(fn GetId
  (return (Variables|Default|GetID)))

(fn UpdateInsightIcon)

(fn SetPointIndex
  (params (PointIndex :type Integer))
  (Variables|Default|SetPointIndex PointIndex))

(fn GetPointIndex
  (return (Variables|Default|GetPointIndex)))