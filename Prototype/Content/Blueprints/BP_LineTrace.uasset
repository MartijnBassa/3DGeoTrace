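; Mouse-driven planning actor that places directional boring points A and B and dirt depots in the world via cursor line traces.
; Alt+click spawns up to two points; the second draws a debug line and computes dirt volume from length, height and width, setting a depot limit.
; Shift+click spawns depots within that limit, choosing variants by remaining dirt.
; PlanWidget and DepotsInterface events toggle placement, and dirt amount is broadcast after Alt+click.
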(event Custom|Place%20Point%20A%20B
  (params (isChecked :type Boolean))
  (Variables|Default|SetisChecked isChecked))

(event Custom|SetDepotType
  (params (DepotType :type EIntTypes%20Enum :default "NewEnumerator4") (isChecked :type Boolean))
  (Variables|Default|SetisCheckedDepot isChecked)
  (Variables|Default|SetdepotType DepotType))

(event EventBeginPlay
  (Utilities|FlowControl|Sequence
    (:then_0
      (Input|EnableInput (Game|GetPlayerController 0)))
    (:then_1
      (Utilities|FlowControl|Delay 0.1)
      (bind _foundwidgets (Widget|GetAllWidgetsOfClass "/Game/UI/PlanWidget.PlanWidget_C" true))
      (EventDispatchers|BindEventtoPlacePointAB _foundwidgets (delegate Custom|Place%20Point%20A%20B)))
    (:then_2
      (Utilities|FlowControl|Delay 0.1)
      (bind _foundwidgets_2 (Widget|GetAllWidgetsOfClass "/Game/UI/DepotsInterface.DepotsInterface_C" true))
      (EventDispatchers|BindEventtoSetAmountOfDepots _foundwidgets_2 (delegate Custom|SetDepotType)))))

(event Collision|EventActorBeginOverlap
  (params (OtherActor :type Actor%20Object%20Reference)))

(event EventTick
  (params (DeltaSeconds :type Float%20%28single-precision%29)))

(event Input|MouseEvents|ShiftLeftMouseButton
  (params (Key :type Key%20Structure))
  (:Pressed
    (CallFunction|PlaceDepot (Variables|Default|GetisCheckedDepot) (Variables|Default|GetdepotType))))

(event Input|MouseEvents|AltLeftMouseButton
  (params (Key :type Key%20Structure))
  (:Pressed
    (CallFunction|PlacePointAB (Variables|Default|GetisChecked))
    (Default|CallSendDirtAmount (Variables|Default|GetamountOfDirt))))

(fn ConstructionScript)

(fn PlacePointAB
  (params (checked :type Boolean))
  (bind _pointarray (Variables|Default|GetpointArray))
  (if checked
    (if (not (>= (Utilities|Array|Length (Variables|Default|GetpointArray)) 2))
      (bind (_linetracevector _hit) (CallFunction|LineTrace))
      (if _hit
        (if (Utilities|Array|IsEmpty (Variables|Default|GetpointArray))
          (bind _output_get (Variables|Default|SetpointA _linetracevector))
          (bind _returnvalue (Game|SpawnActorfromClass "/Game/Blueprints/BP_Directional_Boring.BP_Directional_Boring_C" (Math|Transform|MakeTransform (Math|Vector|MakeVector (.x _output_get) (.y _output_get) (+ (.z _output_get) 45.0)) "0, 0, 0" "1.000000,1.000000,1.000000") "Undefined" 0 true 0))
          (Utilities|Array|Add _pointarray _returnvalue)
          (else
            (bind _output_get_2 (Variables|Default|SetpointB _linetracevector))
            (bind _returnvalue_2 (Game|SpawnActorfromClass "/Game/Blueprints/BP_Directional_Boring.BP_Directional_Boring_C" (Math|Transform|MakeTransform (Math|Vector|MakeVector (.x _output_get_2) (.y _output_get_2) (+ (.z _output_get_2) 45.0)) "0, 0, 0" "1.000000,1.000000,1.000000") "Undefined" 0 false 0))
            (Utilities|Array|Add _pointarray _returnvalue_2)
            (CallFunction|MakeLineBetweenPointAB)))))))

(fn MakeLineBetweenPointAB
  (for _array_element (Variables|Default|GetpointArray)
    (Rendering|Debug|DrawDebugLine :LineStart (Variables|Default|GetpointA) :LineEnd (Variables|Default|GetpointB) :Duration 5e+05 :Thickness 1e+01))
  (CallFunction|CalculateDirtAmount))

(fn ConvertWorldSpace
  (Variables|Default|SetwordSpaceB (Math|Transform|InverseTransformLocation (Math|Conversions|ToTransform(Vector) (Transformation|GetActorLocation)) (Variables|Default|GetwordSpaceB))))

(fn CalculateDirtAmount
  (bind _output_get (Variables|Default|Setlength (/ (Math|Vector|VectorLength (- (Variables|Default|GetpointA) (Variables|Default|GetpointB))) 1e+02)))
  (bind _output_get_2 (Variables|Default|SetamountOfDirt (Math|Conversions|ToFloat(Integer) (Math|Float|Round (* _output_get (Variables|Default|Getheight) (Variables|Default|Getwidth))))))
  (bind _output_get_3 (Variables|Default|SetDirt%20Amount%20Copy _output_get_2))
  (if (<= _output_get_3 (LocalVariables|GetdepotVolume))
    (Variables|Default|SetmaxAllowedDepots 1)
    (else
      (while (> (Variables|Default|GetDirt%20Amount%20Copy) 0.0)
        (Variables|Default|SetmaxAllowedDepots (+ (Variables|Default|GetmaxAllowedDepots) 1))
        (Variables|Default|SetDirt%20Amount%20Copy (- (Variables|Default|GetDirt%20Amount%20Copy) 25.0)))
      (Variables|Default|SetdirtEditable (Variables|Default|GetamountOfDirt)))))

(fn LineTrace
  (bind _returnvalue (Game|GetPlayerController 0))
  (bind (_worldlocation _worlddirection) (Game|Player|ConvertMouseLocationToWorldSpace _returnvalue))
  (bind (_outhit _returnvalue_2) (Collision|LineTraceByChannel _worldlocation (+ _worldlocation (* _worlddirection 1e+05)) "TraceTypeQuery1" true 0 "None"))
  (return (.Location (Collision|BreakHitResult _outhit)) _returnvalue_2))

(fn PlaceDepot
  (params (isChecked :type Boolean) (depotType :type EIntTypes%20Enum :default "NewEnumerator4"))
  (if isChecked
    (if (not (>= (Utilities|Array|Length (Variables|Default|GetdepotArray)) (Variables|Default|GetmaxAllowedDepots)))
      (LocalVariables|Setdepot depotType)
      (bind (_linetracevector _hit) (CallFunction|LineTrace))
      (if _hit
        (bind _output_get (LocalVariables|SetnewLocationContainer (Math|Vector|MakeVector (.x _linetracevector) (.y _linetracevector) (+ (.z _linetracevector) 65.0))))
        (bind _depot (CallFunction|SpawnDepot _output_get))
        (Utilities|Array|Add (Variables|Default|GetdepotArray) _depot)))))

(fn SpawnDepot
  (params (location :type Vector))
  (if (< (Variables|Default|GetdirtEditable) 25.0)
    (bind _returnvalue (Game|SpawnActorfromClass "/Game/Blueprints/BP_DirtDepot.BP_DirtDepot_C" (Math|Transform|MakeTransform location "0, 0, 0" "1.000000,1.000000,1.000000") "Undefined" 0 "NewEnumerator4" 0))
    (return _returnvalue)
    (elif (< (Variables|Default|GetdirtEditable) 5e+01)
      (Game|SpawnActorfromClass "/Game/Blueprints/BP_DirtDepot.BP_DirtDepot_C" (Math|Transform|MakeTransform location "0, 0, 0" "1.000000,1.000000,1.000000") "Undefined" 0 "NewEnumerator5" 0)
      (Variables|Default|SetdirtEditable (- (Variables|Default|GetdirtEditable) 25.0))
      (elif (< (Variables|Default|GetdirtEditable) 75.0)
        (Game|SpawnActorfromClass "/Game/Blueprints/BP_DirtDepot.BP_DirtDepot_C" (Math|Transform|MakeTransform location "0, 0, 0" "1.000000,1.000000,1.000000") "Undefined" 0 "NewEnumerator6" 0)
        (Variables|Default|SetdirtEditable (- (Variables|Default|GetdirtEditable) 25.0))))))